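; Behavior Tree task that selects the next patrol waypoint for an AI-controlled ThirdPersonCharacter.
; It reads the pawn's PatrolPoints array and writes the point at the Blackboard's NextWaypointIndex into the Waypoint key.
; It then increments that index, wrapping by modulo over the array length to loop the route, and finishes successfully.
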(event EventReceiveExecuteAI
  (params (OwnerController :type AI%20Controller%20Object%20Reference) (ControlledPawn :type Pawn%20Object%20Reference))
  (CallFunction|GetWaypoints ControlledPawn)
  (bind (_current_index _length) (CallFunction|SetWaypoint))
  (CallFunction|UpdateNextWaypointIndex _current_index _length)
  (AI|BehaviorTree|FinishExecute true))

(fn GetWaypoints
  (params (Object :type Object%20Object%20Reference))
  (bind _asthird_person_character (Utilities|Casting|CastToThirdPersonCharacter Object))
  (Variables|Default|SetPatrolPoints (Variables|/Game/ThirdPersonCPP/Blueprints/ThirdPersonCharacter.ThirdPersonCharacter_C|GetPatrolPoints _asthird_person_character))
  (return))

(fn SetWaypoint
  (params (ControlledActor :type Actor%20Object%20Reference))
  (bind _patrolpoints (Variables|Default|GetPatrolPoints))
  (bind _nextwaypointindex (Variables|Default|GetNextWaypointIndex))
  (bind _returnvalue (Class|BTFunctionLibrary|GetBlackboardValueasInt _nextwaypointindex))
  (Class|BTFunctionLibrary|SetBlackboardValueasObject (Variables|Default|GetWaypoint) (Utilities|Array|Get(acopy) _patrolpoints _returnvalue))
  (return _returnvalue (Utilities|Array|Length _patrolpoints)))

(fn UpdateNextWaypointIndex
  (params (Current%20Index :type Integer%20%28by%20ref%29) (Length :type Integer))
  (bind _result (Math|Integer|IncrementInt Current%20Index)
    (:%20%20
      (Class|BTFunctionLibrary|SetBlackboardValueasInt (Variables|Default|GetNextWaypointIndex) (Math|Integer|%(Integer) _result Length))
      (return))))